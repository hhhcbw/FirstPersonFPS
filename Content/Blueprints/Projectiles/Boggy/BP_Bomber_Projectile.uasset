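; Bomber projectile Blueprint that explodes when destroyed.
; On BeginPlay it snaps its particle component to the Sparks socket on the mesh.
; Destruction calls Explode, which spawns a small explosion effect and sound, then applies radial damage credited to the owner's AI controller.
; A debug print reports whether the damage call hit anything; overlap and tick events are disabled.
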(event EventBeginPlay
  (|CallParentFunction)
  (Transformation|AttachComponentToComponent (Variables|Default|GetParticle) (Variables|Character|GetMesh) "Sparks" "SnapToTarget" "SnapToTarget" "SnapToTarget" true))

(event Collision|EventActorBeginOverlap
  (params (OtherActor :type Actor%20Object%20Reference))
  (|CallParentFunction OtherActor) ; This node is disabled and will not be called.\nDrag off pins to build functionality.
)

(event EventTick
  (params (DeltaSeconds :type Float%20%28single-precision%29))
  (|CallParentFunction DeltaSeconds) ; This node is disabled and will not be called.\nDrag off pins to build functionality.
)

(event EventDestroyed
  (CallFunction|Explode))

(fn ConstructionScript
  (|CallParentFunction))

(fn Explode
  ;[1 1 1] Emit FX
  (Effects|SpawnEmitteratLocation "/Game/ThirdAsserts/UltimateCharacter/Effects/Projectiles/P_SmallExplosion.P_SmallExplosion" (Transformation|GetActorLocation) (Transformation|GetActorRotation))
  ;[1 1 1] PlaySound
  (Audio|PlaySoundatLocation "/Game/ThirdAsserts/UltimateCharacter/Sounds/Projectiles/Explode_Cue.Explode_Cue" (Transformation|GetActorLocation) "0, 0, 0" 1.0 1.0 0.0 0 0 0)
  ;[1 1 1] Apply Radial Damage
  (bind _returnvalue (Game|Damage|ApplyRadialDamage 25.0 (Transformation|GetActorLocation) 1e+02 0 0 self (AI|GetAIController (Components|GetOwner)) false "ECC_Visibility"))
  (if _returnvalue
    (Development|PrintString "Damage At Least Pawn")
    (else
      (Development|PrintString "Damage No Pawn"))))