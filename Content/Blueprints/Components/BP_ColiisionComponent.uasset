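; BP_ColiisionComponent is a collision component that reports actors overlapping a socket on an assigned primitive component.
; While enabled, Tick runs a 32-unit sphere overlap at FireSocket, filtered to one object type.
; Each new actor joins CollisionActors and fires OnCollide, so it reports only once until the list is cleared.
; It starts disabled, with separate functions to toggle detection, clear the list and set the primitive.
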(event EventBeginPlay
  (CallFunction|ClearCollision)
  (CallFunction|CantCollide))

(event EventTick
  (params (DeltaSeconds :type Float%20%28single-precision%29))
  (if (Variables|Default|GetCanCollision)
    (bind _outactors (Collision|SphereOverlapActors (Transformation|GetSocketLocation (Variables|Default|GetPrimitiveComponent) "FireSocket") 32.0 (Utilities|Array|MakeArray (Utilities|Enum|LiteralenumEObjectTypeQuery "ObjectTypeQuery7")) 0))
    (for _array_element _outactors
      (CallFunction|AddCollisionActor _array_element))))

(fn ClearCollision
  (Utilities|Array|Clear (Variables|Default|GetCollisionActors)))

(fn CanCollide
  (Variables|Default|SetCanCollision true))

(fn CantCollide
  (Variables|Default|SetCanCollision false))

(fn AddCollisionActor
  (params (A :type Actor%20Object%20Reference))
  (if (not (Utilities|Array|ContainsItem (Variables|Default|GetCollisionActors) A))
    (Utilities|Array|Add (Variables|Default|GetCollisionActors) A)
    (Default|CallOnCollide A)))

(fn SetPrimitiveComponent
  (params (PrimComp :type Primitive%20Component%20Object%20Reference))
  (Variables|Default|SetPrimitiveComponent PrimComp))