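; AI-controlled character with health, an attack montage, a patrol point list and an overhead-style state widget.
; Point damage lowers health and updates the widget's health ratio; at zero it stops the brain logic, plays the death montage, then destroys the actor.
; Patrol, Search and Pursuit behaviors map to symbol text on WT_AIState, though BeginPlay casts the same widget to AI_WidgetBP.
; Getters expose attack distance and type.
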(event Custom|OnDead
  (if (not (Variables|Default|GetNew_IsDying))
    (Variables|Default|SetNew_IsDying true)
    (AI|Logic|StopLogic (Variables|/Script/AIModule.AIController|GetBrainComponent (AI|GetAIController self)) "")
    (CallFunction|StopAllMontage)
    (bind _returnvalue (Animation|PlayAnimMontage (Variables|Default|GetDeathAnim) 1.0 "None"))
    (Utilities|FlowControl|Delay _returnvalue)
    (Actor|DestroyActor)))

(event Custom|OnSimpleAttack
  (bind _returnvalue (Animation|PlayAnimMontage (Variables|Default|GetAttackAnim) 1.0 "None"))
  (Utilities|FlowControl|Delay _returnvalue))

(event Custom|CS_AddPatrolPoint
  (params (PatrolPoint :type Actor%20Object%20Reference))
  (Utilities|Array|Add (Variables|AI|GetPatrolPoints) PatrolPoint))

(event EventBeginPlay
  (|CallParentFunction)
  (bind _asai_widget_bp (Utilities|Casting|CastToAI_WidgetBP (UserInterface|GetUserWidgetObject (Variables|Default|GetAIWidget))))
  (Variables|UI|SetUI_AIBehavior _asai_widget_bp))

(event Collision|EventActorBeginOverlap
  (params (OtherActor :type Actor%20Object%20Reference)))

(event EventTick
  (params (DeltaSeconds :type Float%20%28single-precision%29))
  (|CallParentFunction DeltaSeconds) ; This node is disabled and will not be called.\nDrag off pins to build functionality.
)

(event EventUpdateBehaviorWidget
  (params (AIBehavior :type E_AIBehavior%20Enum :default "NewEnumerator0"))
  (bind _aswt_aistate (Utilities|Casting|CastToWT_AIState (UserInterface|GetUserWidgetObject (Variables|Default|GetAIWidget))))
  (switch Utilities|FlowControl|Switch|SwitchonE_AIBehavior AIBehavior
    (:NewEnumerator0
      (Variables|/Game/Blueprints/UMG/WT_AIState.WT_AIState_C|SetAIBehaviorText _aswt_aistate "... ..."))
    (:NewEnumerator1
      (Variables|/Game/Blueprints/UMG/WT_AIState.WT_AIState_C|SetAIBehaviorText _aswt_aistate "??"))
    (:NewEnumerator2
      (Variables|/Game/Blueprints/UMG/WT_AIState.WT_AIState_C|SetAIBehaviorText _aswt_aistate "!!"))))

(event Game|Damage|EventPointDamage
  (params (Damage :type Float%20%28single-precision%29) (DamageType :type Damage%20Type%20Object%20Reference) (HitLocation :type Vector :default "0, 0, 0") (HitNormal :type Vector :default "0, 0, 0") (HitComponent :type Primitive%20Component%20Object%20Reference) (BoneName :type Name :default "None") (ShotFromDirection :type Vector :default "0, 0, 0") (InstigatedBy :type Controller%20Object%20Reference) (DamageCauser :type Actor%20Object%20Reference) (HitInfo :type Hit%20Result%20Structure%20%28by%20ref%29))
  (if (not (or (<= (Variables|New|GetHealthNew) 0.0) (Variables|Default|GetNew_IsDying)))
    (bind _output_get (Variables|New|SetHealthNew (- (Variables|New|GetHealthNew) Damage)))
    (if (<= (Variables|New|GetHealthNew) 0.0)
      (CallFunction|UpdateWidget _output_get)
      (CallFunction|OnDead)
      (else
        (CallFunction|UpdateWidget _output_get)))))

(event Game|Damage|EventAnyDamage
  (params (Damage :type Float%20%28single-precision%29) (DamageType :type Damage%20Type%20Object%20Reference) (InstigatedBy :type Controller%20Object%20Reference) (DamageCauser :type Actor%20Object%20Reference)))

(fn ConstructionScript
  (|CallParentFunction))

(fn UpdateWidget
  (params (A :type Float%20%28single-precision%29))
  (bind _aswt_aistate (Utilities|Casting|CastToWT_AIState (UserInterface|GetUserWidgetObject (Variables|Default|GetAIWidget))))
  (Variables|/Game/Blueprints/UMG/WT_AIState.WT_AIState_C|SetHealth _aswt_aistate (/ A (Variables|New|GetMaxHealthNew))))

(fn GetAttackDistance
  (return (Variables|Default|GetAttackDistance)))

(fn GetAIType
  (return (Variables|Default|GetAttackType)))