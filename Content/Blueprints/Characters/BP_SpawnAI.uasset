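; BP_SpawnAI is a spawner that creates a random mix of Boggy AI enemies at its own transform.
; SpawnAI loops over the requested count, picking Guardian, Slime or Bomber at random, and passes each new AI the spawner's PatrolPoint.
; It clears and refills SpawnAIArray on every call and returns it.
; Its event graph is empty, so spawning runs only when SpawnAI is called.
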(event EventBeginPlay)

(event Collision|EventActorBeginOverlap
  (params (OtherActor :type Actor%20Object%20Reference)))

(event EventTick
  (params (DeltaSeconds :type Float%20%28single-precision%29)))

(fn ConstructionScript)

(fn SpawnAI
  (params (AICount :type Integer))
  (bind _returnvalue (Transformation|GetActorTransform))
  (Utilities|Array|Clear (Variables|Default|GetSpawnAIArray))
  (for _index (range 0 AICount)
    (switch int (Math|Random|RandomInteger 3)
      (:0
        (bind _returnvalue_2 (Game|SpawnActorfromClass "/Game/Blueprints/Characters/Boggy/BP_AI_GuardianBoggy_2.BP_AI_GuardianBoggy_2_C" _returnvalue "Undefined" 0 0 0))
        (Default|CSAddPatrolPoint _returnvalue_2 (Variables|Default|GetPatrolPoint))
        (Utilities|Array|Add (Variables|Default|GetSpawnAIArray) _returnvalue_2))
      (:1
        (bind _returnvalue_3 (Game|SpawnActorfromClass "/Game/Blueprints/Characters/Boggy/BP_AI_SlimeBoggy.BP_AI_SlimeBoggy_C" _returnvalue "Undefined" 0 0 0))
        (Default|CSAddPatrolPoint _returnvalue_3 (Variables|Default|GetPatrolPoint))
        (Utilities|Array|Add (Variables|Default|GetSpawnAIArray) _returnvalue_3))
      (:2
        (bind _returnvalue_4 (Game|SpawnActorfromClass "/Game/Blueprints/Characters/Boggy/BP_AI_BomberBoggy.BP_AI_BomberBoggy_C" _returnvalue "Undefined" 0 0 0))
        (Default|CSAddPatrolPoint _returnvalue_4 (Variables|Default|GetPatrolPoint))
        (Utilities|Array|Add (Variables|Default|GetSpawnAIArray) _returnvalue_4))))
  (return (Variables|Default|GetSpawnAIArray)))