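; BP_AI_BomberBoggy is an AI Boggy enemy variant that attacks by launching bomber projectiles.
; On BeginPlay it binds a handler to the DoSimpleAttack event.
; The handler spawns BP_Bomber_Projectile at the mesh's right weapon socket with the actor's rotation, setting itself as owner and instigator.
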(event Custom|DoSimpleAttack_Event
  (bind _self self)
  (Game|SpawnActorfromClass "/Game/Blueprints/Projectiles/Boggy/BP_Bomber_Projectile.BP_Bomber_Projectile_C" (Math|Transform|MakeTransform (Transformation|GetSocketLocation (Variables|Character|GetMesh) "Weapon_R_Socket") (Transformation|GetActorRotation)) "Undefined" _self _self))

(event EventBeginPlay
  (EventDispatchers|BindEventtoDoSimpleAttack (delegate Custom|DoSimpleAttack_Event)))

(event EventTick
  (params (DeltaSeconds :type Float%20%28single-precision%29))
  (|CallParentFunction DeltaSeconds) ; This node is disabled and will not be called.\nDrag off pins to build functionality.
)

(fn ConstructionScript
  (|CallParentFunction))