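; AI slime variant of the Boggy character that performs its simple attack by spitting a slime projectile.
; On BeginPlay it runs the parent logic, then binds a handler to the DoSimpleAttack dispatcher.
; The handler spawns BP_SlimeProjetile at the mesh's Mouth_Socket, facing the actor's rotation, with itself as owner and instigator.
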(event Custom|DoSimpleAttack_Event
  (bind _self self)
  (Game|SpawnActorfromClass "/Game/Blueprints/Projectiles/Boggy/BP_SlimeProjetile.BP_SlimeProjetile_C" (Math|Transform|MakeTransform (Transformation|GetSocketLocation (Variables|Character|GetMesh) "Mouth_Socket") (Transformation|GetActorRotation)) "Undefined" _self _self))

(event EventBeginPlay
  (|CallParentFunction)
  (EventDispatchers|BindEventtoDoSimpleAttack (delegate Custom|DoSimpleAttack_Event)))

(event Collision|EventActorBeginOverlap
  (params (OtherActor :type Actor%20Object%20Reference))
  (|CallParentFunction OtherActor) ; This node is disabled and will not be called.\nDrag off pins to build functionality.
)

(event EventTick
  (params (DeltaSeconds :type Float%20%28single-precision%29))
  (|CallParentFunction DeltaSeconds) ; This node is disabled and will not be called.\nDrag off pins to build functionality.
)

(fn ConstructionScript
  (|CallParentFunction))